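; BP_SetupScene is a demo scene controller that toggles between two placed mesh actors, GlintMesh and NoGlintMesh, apparently to compare a glint effect on and off.
; On BeginPlay it enables input from player 0.
; Caps Lock flip-flops which of the two actors is visible.
; Tab flip-flops both actors' static mesh between a big plane and the ocean mesh, so the comparison works on either surface.
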(event `self.ReceiveBeginPlay`
  (`self.EnableInput` (`GameplayStatics.GetPlayerController` 0)))

(event `Key|CapsLock`
  (params (Key :type "Key Structure"))
  (bind _glintmesh (`self.GlintMesh`))
  (bind _noglintmesh (`self.NoGlintMesh`))
  (:`Pressed`
    (`/Engine/EditorBlueprintResources/StandardMacros.FlipFlop`
      (:`A`
        (`self.SetActorHiddenInGame` _glintmesh true)
        (`self.SetActorHiddenInGame` _noglintmesh false))
      (:`B`
        (`self.SetActorHiddenInGame` _glintmesh false)
        (`self.SetActorHiddenInGame` _noglintmesh true)))))

(event `Key|Tab`
  (params (Key :type "Key Structure"))
  (bind _staticmeshcomponent (`StaticMeshActor.StaticMeshComponent` (`self.NoGlintMesh`)))
  (bind _staticmeshcomponent_2 (`StaticMeshActor.StaticMeshComponent` (`self.GlintMesh`)))
  (:`Pressed`
    (`/Engine/EditorBlueprintResources/StandardMacros.FlipFlop`
      (:`A`
        (`StaticMeshComponent.SetStaticMesh` _staticmeshcomponent_2 "/Game/Models/SM_BigPlane.SM_BigPlane")
        (`StaticMeshComponent.SetStaticMesh` _staticmeshcomponent "/Game/Models/SM_BigPlane.SM_BigPlane"))
      (:`B`
        (`StaticMeshComponent.SetStaticMesh` _staticmeshcomponent_2 "/Game/Models/ocean.ocean")
        (`StaticMeshComponent.SetStaticMesh` _staticmeshcomponent "/Game/Models/ocean.ocean")))))

(fn `UserConstructionScript`)