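; Player controller that jumps the player pawn between preset viewpoints in the scene using number keys 0 to 5.
; On BeginPlay it finds the BP_SetupScene actor, whose Anchors array supplies the target transforms.
; GoToAnchor moves the pawn to the chosen anchor's location and sets control rotation to match.
; Anchor 0 leaves look input free, while the other anchors lock it via SetIgnoreLookInput.
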(event `self.ReceiveBeginPlay`
  (bind _returnvalue (`GameplayStatics.GetActorOfClass` "/Game/Blueprints/BP_SetupScene.BP_SetupScene_C"))
  (set `self.SetupSceneActor` _returnvalue))

(event `Key|Zero`
  (params (Key :type "Key Structure"))
  (:`Pressed`
    (`self.GoToAnchor` 0)
    (`self.SetInputLocked` false)))

(event `Key|One`
  (params (Key :type "Key Structure"))
  (:`Pressed`
    (`self.GoToAnchor` 1)
    (`self.SetInputLocked` true)))

(event `Key|Two`
  (params (Key :type "Key Structure"))
  (:`Pressed`
    (`self.GoToAnchor` 2)
    (`self.SetInputLocked` true)))

(event `Key|Three`
  (params (Key :type "Key Structure"))
  (:`Pressed`
    (`self.GoToAnchor` 3)
    (`self.SetInputLocked` true)))

(event `Key|Four`
  (params (Key :type "Key Structure"))
  (:`Pressed`
    (`self.GoToAnchor` 4)
    (`self.SetInputLocked` true)))

(event `Key|Five`
  (params (Key :type "Key Structure"))
  (:`Pressed`
    (`self.GoToAnchor` 5)
    (`self.SetInputLocked` true)))

(fn `GoToAnchor`
  (params (Index :type Integer))
  (bind (_returnvalue_location _returnvalue_rotation) (`KismetMathLibrary.BreakTransform` (`self.GetTransform` (`|GetArrayItem` (`/Game/Blueprints/BP_SetupScene.Anchors` (`self.SetupSceneActor`)) Index))))
  (`self.K2_SetActorLocation` (`GameplayStatics.GetPlayerPawn` 0) _returnvalue_location false false)
  (`self.SetControlRotation` _returnvalue_rotation))

(fn `SetInputLocked`
  (params (Value :type Boolean))
  (`self.SetIgnoreLookInput` Value))

(fn `UserConstructionScript`)